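; BP_Enemy_Base is a base enemy character that provides chase, sword combat, movement speed and patrol route functions.
; Attack, WieldSword and SheathSword play montages and fire dispatchers on completion, with interruptions signalling conditionally for wield and sheath.
; Montage notifies spawn and socket-attach the sword or destroy it, updating IsWieldingSword.
; ChasePlayer moves toward the player pawn, and SetMovementSpeed maps a speed state to walk speed.
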(event `self.ReceiveBeginPlay`)

(event `ChasePlayer`
  (`|AIMoveTo` self (0.0 0.0 0.0) (`GameplayStatics.GetPlayerPawn` 0) 150.0))

(event `Attack`
  (`|PlayMontage` (`self.Mesh`) "/Game/Animations/Melee/sword-slash_Montage.sword-slash_Montage"
    (:`OnCompleted`
      _)
    (:`OnInterrupted`
      _))
  (`self.OnAttackFinished`))

(event `WieldSword`
  (bind _notifyname (`|PlayMontage` (`self.Mesh`) "/Game/Animations/Melee/sword-wield_Montage.sword-wield_Montage")
    (:`OnCompleted`
      (`self.OnWieldSword` :!label _label))
    (:`OnInterrupted`
      (if (`self.IsWieldingSword`)
        (goto _label)))
    (:`OnNotifyBegin`
      (switch `name` _notifyname
        (:`WieldSword`
          (bind _returnvalue (`|SpawnActorFromClass` "/Game/AI/BP_Sword.BP_Sword_C" (`KismetMathLibrary.MakeTransform` (0.0 0.0 0.0)) "Undefined" "MultiplyWithRoot" null null))
          (bind _output_get (set `self.Sword` _returnvalue))
          (`self.K2_AttachToComponent` _output_get (`self.Mesh`) (`self.SwordSocketName`) "SnapToTarget" "SnapToTarget" "KeepWorld" true)
          (set `self.IsWieldingSword` true))))))

(event `/Game/AI/BPI_Enemy.SetMovementSpeed`
  (params (SpeedState :type "/Game/AI/E_MovementSpeed Enum" :default "NewEnumerator0"))
  (set `CharacterMovementComponent.MaxWalkSpeed` (select `/Game/AI/E_MovementSpeed` SpeedState :`NewEnumerator1` 100.0 :`NewEnumerator2` 300.0 :`NewEnumerator3` 500.0 :!type "Float (single-precision)") (`self.CharacterMovement`)))

(event `SheathSword`
  (bind _notifyname (`|PlayMontage` (`self.Mesh`) "/Game/Animations/Melee/sword-sheath_Montage.sword-sheath_Montage")
    (:`OnCompleted`
      (`self.OnSheathSword` :!label _label_2))
    (:`OnInterrupted`
      (if (not (`self.IsWieldingSword`))
        (goto _label_2)))
    (:`OnNotifyBegin`
      (switch `name` _notifyname
        (:`DropSword`
          (set `self.IsWieldingSword` false)
          (`self.K2_DestroyActor` (`self.Sword`)))))))

(fn `GetPatrolRoute`
  (returns (Route :type "/Game/AI/BP_PatrolRoute Object Reference"))
  (return (`self.PatrolRoute`)))

(fn `UserConstructionScript`)